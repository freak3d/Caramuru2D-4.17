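; A 2D tilemap trigger actor that saves the player's position as a checkpoint or save point.
; When an actor tagged Caramuru overlaps, it creates a fresh Save_Info, writes the player character's location to it, saves once to slot "Loc", and prints the location.
; The construction script sizes the box from ChangeHitBox and picks the billboard sprite by the CheckPoint flag; both modes save identically.
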(event `self.ReceiveActorBeginOverlap`
  (params (OtherActor :type "Actor Object Reference"))
  (bind _saveinfo (`self.SaveInfo`))
  (bind (_returnvalue_x _returnvalue_y _returnvalue_z) (`KismetMathLibrary.BreakVector` (`self.K2_GetActorLocation` (`self.CharInfo`))))
  (bind (_returnvalue_x_2 _returnvalue_y_2 _returnvalue_z_2) (`KismetMathLibrary.BreakVector` (`self.K2_GetActorLocation` (`self.CharInfo`))))
  (if (`self.ActorHasTag` OtherActor "Caramuru")
    (bind _returnvalue (`GameplayStatics.CreateSaveGameObject` "/Game/Resources/2dtiledmap/CheckPoint/Save_Info.Save_Info_C"))
    (bind _assave_info (cast `/Game/Resources/2dtiledmap/CheckPoint/Save_Info` _returnvalue))
    (set `self.SaveInfo` _assave_info)
    (bind _ascaramuru (cast `/Game/Resources/Blueprints/Character/Caramuru` (`GameplayStatics.GetPlayerCharacter` 0)))
    (set `self.CharInfo` _ascaramuru)
    (if (`self.CheckPoint`)
      (`/Engine/EditorBlueprintResources/StandardMacros.DoOnce` false
        (:`Completed`
          (set `/Game/Resources/2dtiledmap/CheckPoint/Save_Info.CheckLocation` (`KismetMathLibrary.MakeVector` _returnvalue_x_2 _returnvalue_y_2 _returnvalue_z_2) (`self.SaveInfo`))
          (`GameplayStatics.SaveGameToSlot` _saveinfo "Loc")))
      (else
        (`/Engine/EditorBlueprintResources/StandardMacros.DoOnce` false
          (:`Completed`
            (set `/Game/Resources/2dtiledmap/CheckPoint/Save_Info.CheckLocation` (`KismetMathLibrary.MakeVector` _returnvalue_x _returnvalue_y _returnvalue_z) (`self.SaveInfo`))
            (`GameplayStatics.SaveGameToSlot` _saveinfo "Loc")))))
    (`KismetSystemLibrary.PrintString` (`KismetStringLibrary.Conv_VectorToString` (`/Game/Resources/2dtiledmap/CheckPoint/Save_Info.CheckLocation` (`self.SaveInfo`))))))

(fn `UserConstructionScript`
  (`BoxComponent.SetBoxExtent` (`self.Box`) (`self.ChangeHitBox`) true)
  (if (`self.CheckPoint`)
    (`BillboardComponent.SetSprite` (`self.Billboard`) "/Game/Resources/2dtiledmap/CheckPoint/CheckPoint.CheckPoint")
    (else
      (`BillboardComponent.SetSprite` (`self.Billboard`) "/Game/Resources/2dtiledmap/CheckPoint/SavePoint.SavePoint"))))