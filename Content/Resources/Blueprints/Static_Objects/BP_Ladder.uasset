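; BP_Ladder is a climbable ladder (with a vine-climbing sound) that the player ascends by holding U.
; Tick measures only the X-axis distance to player 0, flags OnLadder within a narrow range, and enables input in either case.
; Pressing U in range starts a Delay-based loop that sets Flying, plays the sound and adds upward movement input.
; Releasing U or leaving range restores Walking on the next loop pass.
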(event `self.ReceiveTick`
  (params (DeltaSeconds :type "Float (single-precision)"))
  (bind _returnvalue_x (`KismetMathLibrary.BreakVector` (`self.K2_GetActorLocation`)))
  (bind _returnvalue (`GameplayStatics.GetPlayerController` 0))
  (bind _returnvalue_x_2 (`KismetMathLibrary.BreakVector` (`self.K2_GetActorLocation` (`GameplayStatics.GetPlayerCharacter` 0))))
  (`|ExecutionSequence`
    (:`then_0`
      (set `self.DisLadder` (- _returnvalue_x _returnvalue_x_2)))
    (:`then_1`
      (if (`KismetMathLibrary.InRange_FloatFloat` (`self.DisLadder`) -20.0 20.0 false)
        (set `self.OnLadder` true)
        (`self.EnableInput` _returnvalue)
        (else
          (set `self.OnLadder` false)
          (`self.EnableInput` _returnvalue))))))

(event `Key|U`
  (params (Key :type "Key Structure"))
  (bind _returnvalue (`GameplayStatics.GetPlayerPawn` 0))
  (bind _returnvalue_location (`KismetMathLibrary.BreakTransform` (`self.GetTransform` _returnvalue)))
  (:`Pressed`
    (if (`KismetMathLibrary.InRange_FloatFloat` (`self.DisLadder`) -20.0 20.0 false)
      (if (`self.OnLadder`) :!label _label
        (if (`PlayerController.IsInputKeyDown` (`GameplayStatics.GetPlayerController` 0) "U")
          (`CharacterMovementComponent.SetMovementMode` (`Character.CharacterMovement` (`GameplayStatics.GetPlayerCharacter` 0)) "MOVE_Flying" 0)
          (`GameplayStatics.PlaySoundAtLocation` "/Game/Sounds/CUE_VineClimbing.CUE_VineClimbing" _returnvalue_location)
          (`Pawn.AddMovementInput` _returnvalue (`self.GetActorUpVector` _returnvalue) (`self.MovementSpeed`) false)
          (`KismetSystemLibrary.Delay` 0.2)
          (goto _label)
          (else
            _)))
      (`CharacterMovementComponent.SetMovementMode` (`Character.CharacterMovement` (`GameplayStatics.GetPlayerCharacter` 0)) "MOVE_Walking" 0))))

(fn `UserConstructionScript`)