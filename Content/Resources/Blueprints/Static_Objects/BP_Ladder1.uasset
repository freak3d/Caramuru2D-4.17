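; Climbable ladder actor that lets the Caramuru character climb and controls its shoot, jump and move abilities.
; The Box volume toggles climbing and ends an active climb on exit.
; Top and Down triggers enable climbing and set edge flags, which Tick uses to re-enable shooting, jumping and movement.
; TopBlock stops blocking pawns inside the Box or while S is held, and blocks again on Box exit.
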(event `self.ReceiveTick`
  (params (DeltaSeconds :type "Float (single-precision)"))
  (`|ExecutionSequence`
    (:`then_0`
      ;[1 1 1] Collide Edge Event
      (if (`self.isTop`)
        (bind _ascaramuru (cast `/Game/Resources/Blueprints/Character/Caramuru` (`GameplayStatics.GetPlayerPawn` 0)))
        (set `/Game/Resources/Blueprints/Character/Caramuru.isShoot` true _ascaramuru)
        (set `/Game/Resources/Blueprints/Character/Caramuru.canJump_0` true _ascaramuru)
        (set `/Game/Resources/Blueprints/Character/Caramuru.canMove` true _ascaramuru)))
    (:`then_1`
      (if (`self.isDown`)
        (bind _ascaramuru_2 (cast `/Game/Resources/Blueprints/Character/Caramuru` (`GameplayStatics.GetPlayerPawn` 0)))
        (set `/Game/Resources/Blueprints/Character/Caramuru.isShoot` true _ascaramuru_2)
        (set `/Game/Resources/Blueprints/Character/Caramuru.canJump_0` true _ascaramuru_2)
        (set `/Game/Resources/Blueprints/Character/Caramuru.canMove` true _ascaramuru_2)))
    (:`then_2`
      ;[1 1 1] Climb Top
      (if (`PlayerController.IsInputKeyDown` (`GameplayStatics.GetPlayerController` 0) "S")
        (`PrimitiveComponent.SetCollisionResponseToChannel` (`self.TopBlock`) "ECC_Pawn" "ECR_Overlap")))))

(event `self.Box.OnComponentBeginOverlap`
  (params (OverlappedComponent :type "PrimitiveComponent Object Reference") (OtherActor :type "Actor Object Reference") (OtherComp :type "PrimitiveComponent Object Reference") (OtherBodyIndex :type Integer) (bFromSweep :type Boolean) (SweepResult :type "HitResult Structure (by ref)"))
  ;[1 1 1] Box Event
  (bind _ascaramuru (cast `/Game/Resources/Blueprints/Character/Caramuru` OtherActor))
  (set `/Game/Resources/Blueprints/Character/Caramuru.canClimb` true _ascaramuru)
  (`PrimitiveComponent.SetCollisionResponseToChannel` (`self.TopBlock`) "ECC_Pawn" "ECR_Overlap"))

(event `self.Box.OnComponentEndOverlap`
  (params (OverlappedComponent :type "PrimitiveComponent Object Reference") (OtherActor :type "Actor Object Reference") (OtherComp :type "PrimitiveComponent Object Reference") (OtherBodyIndex :type Integer))
  ;[1 1 1] Box Event
  (bind _ascaramuru (cast `/Game/Resources/Blueprints/Character/Caramuru` OtherActor))
  (set `/Game/Resources/Blueprints/Character/Caramuru.canClimb` false _ascaramuru)
  (set `/Game/Resources/Blueprints/Character/Caramuru.isShoot` true _ascaramuru)
  (set `/Game/Resources/Blueprints/Character/Caramuru.canJump_0` true _ascaramuru)
  (if (`/Game/Resources/Blueprints/Character/Caramuru.isClimb` _ascaramuru)
    (`/Game/Resources/Blueprints/Character/Caramuru.ClimbEnd` _ascaramuru))
  (`PrimitiveComponent.SetCollisionResponseToChannel` (`self.TopBlock`) "ECC_Pawn" "ECR_Block")
  (set `/Game/Resources/Blueprints/Character/Caramuru.canMove` true _ascaramuru))

(event `self.Top.OnComponentBeginOverlap`
  (params (OverlappedComponent :type "PrimitiveComponent Object Reference") (OtherActor :type "Actor Object Reference") (OtherComp :type "PrimitiveComponent Object Reference") (OtherBodyIndex :type Integer) (bFromSweep :type Boolean) (SweepResult :type "HitResult Structure (by ref)"))
  ;[1 1 1] Top Event
  (bind _ascaramuru (cast `/Game/Resources/Blueprints/Character/Caramuru` OtherActor))
  (set `/Game/Resources/Blueprints/Character/Caramuru.canClimb` true _ascaramuru)
  (set `self.isTop` true)
  ;[1 1 1] Jump Event
  (set `/Game/Resources/Blueprints/Character/Caramuru.canJump_0` true _ascaramuru :!label _label)
  (set `/Game/Resources/Blueprints/Character/Caramuru.CaramuruStates` "NewEnumerator0" _ascaramuru))

(event `self.Top.OnComponentEndOverlap`
  (params (OverlappedComponent :type "PrimitiveComponent Object Reference") (OtherActor :type "Actor Object Reference") (OtherComp :type "PrimitiveComponent Object Reference") (OtherBodyIndex :type Integer))
  ;[1 1 1] Top Event
  (cast `/Game/Resources/Blueprints/Character/Caramuru` OtherActor)
  (set `self.isTop` false))

(event `self.Down.OnComponentBeginOverlap`
  (params (OverlappedComponent :type "PrimitiveComponent Object Reference") (OtherActor :type "Actor Object Reference") (OtherComp :type "PrimitiveComponent Object Reference") (OtherBodyIndex :type Integer) (bFromSweep :type Boolean) (SweepResult :type "HitResult Structure (by ref)"))
  ;[1 1 1] Down Event
  (bind _ascaramuru (cast `/Game/Resources/Blueprints/Character/Caramuru` OtherActor))
  (set `/Game/Resources/Blueprints/Character/Caramuru.canClimb` true _ascaramuru)
  (set `self.isDown` true)
  (goto _label))

(event `self.Down.OnComponentEndOverlap`
  (params (OverlappedComponent :type "PrimitiveComponent Object Reference") (OtherActor :type "Actor Object Reference") (OtherComp :type "PrimitiveComponent Object Reference") (OtherBodyIndex :type Integer))
  ;[1 1 1] Down Event
  (bind _ascaramuru (cast `/Game/Resources/Blueprints/Character/Caramuru` OtherActor))
  (set `/Game/Resources/Blueprints/Character/Caramuru.isShoot` false _ascaramuru)
  (set `self.isDown` false))

(fn `UserConstructionScript`)