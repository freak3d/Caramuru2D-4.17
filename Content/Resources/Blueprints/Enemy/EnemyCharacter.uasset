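; Side-scrolling flipbook enemy that moves horizontally, attacks the Caramuru player and spawns an experience sphere on death.
; Tick updates animation, facing and movement, using player proximity checks to halt movement, enable attacking and turn toward the player.
; Attack launches a force-driven lunge that damages the player on capsule hit; other collisions can reverse direction.
; The angry-chase logic is disconnected, leaving AngryState empty.
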(event `Attack`
  ;[1 0.07227 0.9647] Battle System
  ;;[1 1 1] Attack System
  (if (`self.canAttack`)
    (if (`self.isAttacking`)
      (`KismetSystemLibrary.Delay` (`self.intervalBetweenAttacks`))
      (set `self.isAttacking` false)
      (else
        (`CharacterMovementComponent.AddForce` (`self.CharacterMovement`) (* (`self.directionEnemy`) 20000000.0))
        (set `self.isAttacking` true)))
    (else
      (set `self.isAttacking` false))))

(event `UpdateAnimation`
  ;[0 1 1] Update Animation
  (switch `/Game/Caramuru-States` (`self.BatStates`)
    (:`NewEnumerator1`
      (`PaperFlipbookComponent.SetFlipbook` (`self.Sprite`) "/Game/Resources/2dtiledmap/Enemy/EnemyFlying/FLYING1_Enemy.FLYING1_Enemy"))
    (:`NewEnumerator7`
      (`PaperFlipbookComponent.SetFlipbook` (`self.Sprite`) "/Game/Resources/2dtiledmap/Enemy/Bradador/ENEMY_BradadorMov.ENEMY_BradadorMov"))))

(event `AngryState`
  ;[1 0.07227 0.9647] Battle System
  ;;[1 1 1] Angry State
)

(event `Movement Near Enemy`
  (bind _capsulecomponent (`self.CapsuleComponent`))
  ;[1 0.07227 0.9647] Battle System
  ;;[1 1 1] Movement Near Follow Player
  (if (`self.isNear`)
    (set `self.isWait` true)
    (set `self.canAttack` true)
    (bind _ascaramuru (cast `/Game/Resources/Blueprints/Character/Caramuru` (`GameplayStatics.GetPlayerPawn` 0)))
    (if (`/Game/Resources/Blueprints/Character/Caramuru.isjumping` _ascaramuru)
      (bind _capsulecomponent_2 (`Character.CapsuleComponent` _ascaramuru))
      (if (`self.IsBack` _capsulecomponent_2 _capsulecomponent) :!label _label
        (set `self.bisMovingRight` false)
        (else
          (set `self.bisMovingRight` true)))
      (elif (`self.isDown` _capsulecomponent_2 _capsulecomponent)
        (goto _label)
        (else
          (set `self.isNear` false))))
    (else
      (set `self.isWait` false)
      (set `self.canAttack` false))))

(event `self.ReceiveTick`
  (params (DeltaSeconds :type "Float (single-precision)"))
  ;[0 0 1] Update
  (`self.AngryState`)
  (`self.UpdateAnimation`)
  (`self.Direction`)
  (`self.Near player`)
  (`self.Movement Near Enemy`))

(event `Near player`
  ;[1 0.07227 0.9647] Battle System
  ;;[1 1 1] Is Near Follow Player
  (bind _ascaramuru (cast `/Game/Resources/Blueprints/Character/Caramuru` (`GameplayStatics.GetPlayerPawn` 0)))
  (if (`self.DistancePlayer` _ascaramuru (`self.distance`))
    (set `self.isNear` true)
    (set `self.attackMode` true)
    (else
      (set `self.isNear` false)
      (set `self.attackMode` false)
      (`self.not Follow`))))

(event `Direction`
  (bind _returnvalue (`KismetMathLibrary.SelectVector` (1.0 0.0 0.0) (-1.0 0.0 0.0) (`self.bisMovingRight`)))
  ;[1 1 0] Direction
  (`SceneComponent.K2_SetRelativeRotation` (`self.Sprite`) (`KismetMathLibrary.MakeRotator` 0.0 0.0 (`KismetMathLibrary.SelectFloat` 0.0 180.0 (`self.bisMovingRight`))) false false)
  (set `self.directionEnemy` _returnvalue)
  (`SceneComponent.K2_AddLocalOffset` (`self.CapsuleComponent`) (`KismetMathLibrary.MakeVector` (`KismetMathLibrary.SelectFloat` 0.0 (* (.x _returnvalue) (`self.velocityEnemy`)) (`self.isWait`))) false false))

(event `self.CapsuleComponent.OnComponentHit`
  (params (HitComponent :type "PrimitiveComponent Object Reference") (OtherActor :type "Actor Object Reference") (OtherComp :type "PrimitiveComponent Object Reference") (NormalImpulse :type "Vector Structure") (Hit :type "HitResult Structure (by ref)"))
  ;[1 0 0] Hit
  (`|ExecutionSequence`
    (:`then_0`
      (cast `/Game/Resources/Blueprints/Character/Caramuru` OtherActor)
      (set `self.isCollidePlayer` true))
    (:`then_1`
      (if (`self.isAttacking`)
        (bind _ascaramuru (cast `/Game/Resources/Blueprints/Character/Caramuru` OtherActor))
        (`/Game/Resources/Blueprints/Character/Caramuru.Hit` _ascaramuru (- (`/Game/Resources/Blueprints/Character/Caramuru.Life` _ascaramuru) 10.0))
        (else
          (`KismetSystemLibrary.Delay` 0.1)
          (if (`self.isCollidePlayer`)
            (set `self.isCollidePlayer` false)
            (elif (not (`self.isDamagePlayer`))
              (set `self.isFollow` false)
              (set `self.bisMovingRight` (not (`self.bisMovingRight`))))))))))

(event `Not Follow`
  ;[1 0.07227 0.9647] Battle System
  ;;[1 1 1] Is Not Follow
  (set `self.isNear` false)
  (`KismetSystemLibrary.Delay` 0.5)
  (set `self.isFollow` false))

(event `DMG_Enemy`
  (params (DMG_Taken :type Integer))
  ;[0 0 0] Hit/Dead
  (set `self.isHited` true)
  (set `self.isDamagePlayer` true)
  (bind _output_get (set `self.EnemyHealth` (- (`self.EnemyHealth`) DMG_Taken)))
  (if (<= _output_get 0)
    (`self.K2_DestroyActor`)
    (`|SpawnActorFromClass` "/Game/Resources/Blueprints/ExpSphereActor.ExpSphereActor_C" (`KismetMathLibrary.MakeTransform` (`self.K2_GetActorLocation`)) "Undefined" "OverrideRootScale" null null)
    (else
      (`KismetSystemLibrary.PrintString` (`KismetStringLibrary.Conv_IntToString` (`self.EnemyHealth`)))
      (`KismetSystemLibrary.Delay` 1.0)
      (set `self.isDamagePlayer` false))))

(fn `UserConstructionScript`)