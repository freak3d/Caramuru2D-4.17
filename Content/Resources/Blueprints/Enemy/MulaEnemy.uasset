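; Flying 2D enemy that patrols along the X axis, homes in on the Caramuru player and damages them on contact.
; Tick drives animation, movement and proximity checks, steering toward a nearby player who is jumping or not above it.
; Any capsule hit reverses direction and briefly suspends following.
; Damage reduces health until death, which destroys the enemy and spawns an experience sphere.
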(event `Movement Near Enemy`
  (bind _capsulecomponent (`self.CapsuleComponent`))
  ;[1 0.07227 0.9647] Battle System
  ;;[1 1 1] Movement Near Player
  (if (`self.isNear`)
    (bind _ascaramuru (cast `/Game/Resources/Blueprints/Character/Caramuru` (`GameplayStatics.GetPlayerPawn` 0)))
    (if (`/Game/Resources/Blueprints/Character/Caramuru.isjumping` _ascaramuru)
      (bind _capsulecomponent_2 (`Character.CapsuleComponent` _ascaramuru))
      (if (`self.IsBack` _capsulecomponent_2 _capsulecomponent) :!label _label
        (set `self.bisMovingRight` false)
        (else
          (set `self.bisMovingRight` true)))
      (elif (`self.isDown` _capsulecomponent_2 _capsulecomponent)
        (goto _label)
        (else
          (set `self.isNear` false))))))

(event `UpdateAnimation`
  ;[0 1 1] Update Animation
  (`PaperFlipbookComponent.SetFlipbook` (`self.Sprite`) "/Game/Resources/2dtiledmap/Enemy/EnemyFlying/FLYING1_Enemy.FLYING1_Enemy"))

(event `self.ReceiveTick`
  (params (DeltaSeconds :type "Float (single-precision)"))
  ;[0 0 1] Update
  (`self.UpdateAnimation`)
  (`self.Direction`)
  (`self.Near player`)
  (`self.Movement Near Enemy`))

(event `Near player`
  ;[1 0.07227 0.9647] Battle System
  ;;[1 1 1] is Near Player
  (if (`self.isFollow`)
    (bind _ascaramuru (cast `/Game/Resources/Blueprints/Character/Caramuru` (`GameplayStatics.GetPlayerPawn` 0)))
    (if (`/Game/Resources/Blueprints/Character/Caramuru.isHit` _ascaramuru)
      (set `self.isNear` false)
      (elif (`self.DistancePlayer` _ascaramuru (`self.distance`))
        (set `self.isNear` true)
        (else
          (set `self.isNear` false))))
    (else
      (`self.not Follow`))))

(event `Direction`
  ;[1 1 0] Direction
  (`SceneComponent.K2_SetRelativeRotation` (`self.Sprite`) (`KismetMathLibrary.MakeRotator` 0.0 0.0 (`KismetMathLibrary.SelectFloat` 0.0 180.0 (`self.bisMovingRight`))) false false)
  (`self.AddMovementInput` (`KismetMathLibrary.SelectVector` (1.0 0.0 0.0) (-1.0 0.0 0.0) (`self.bisMovingRight`))))

(event `self.CapsuleComponent.OnComponentHit`
  (params (HitComponent :type "PrimitiveComponent Object Reference") (OtherActor :type "Actor Object Reference") (OtherComp :type "PrimitiveComponent Object Reference") (NormalImpulse :type "Vector Structure") (Hit :type "HitResult Structure (by ref)"))
  ;[1 0 0] Hit Player
  (set `self.isFollow` false)
  (set `self.bisMovingRight` (not (`self.bisMovingRight`)))
  (bind _ascaramuru (cast `/Game/Resources/Blueprints/Character/Caramuru` OtherActor))
  (`/Game/Resources/Blueprints/Character/Caramuru.Hit` _ascaramuru (- (`/Game/Resources/Blueprints/Character/Caramuru.Life` _ascaramuru) 10.0)))

(event `Not Follow`
  ;[1 0.07227 0.9647] Battle System
  ;;[1 1 1] is Not Follow
  (set `self.isNear` false)
  (`KismetSystemLibrary.Delay` 0.5)
  (set `self.isFollow` true))

(event `DMG_Enemy`
  (params (DMG_Taken :type Integer))
  (bind _output_get (set `self.EnemyHealth` (- (`self.EnemyHealth`) DMG_Taken)))
  (if (<= _output_get 0)
    (`self.K2_DestroyActor`)
    (`|SpawnActorFromClass` "/Game/Resources/Blueprints/ExpSphereActor.ExpSphereActor_C" (`KismetMathLibrary.Conv_VectorToTransform` (`self.K2_GetActorLocation`)) "Undefined" "OverrideRootScale" null null)
    (else
      (`KismetSystemLibrary.PrintString` (`KismetStringLibrary.Conv_IntToString` (`self.EnemyHealth`))))))

(fn `UserConstructionScript`)