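; Locked door map object that the player, the Caramuru pawn, opens by spending a key.
; Its Overlap component toggles a flag, and Tick polls the pawn's press input while that flag is set.
; With a key, it decrements the count, destroys itself and plays an unlock sound at world origin.
; Without one, it prints a Portuguese no-key message.
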(event `self.ReceiveTick`
  (params (DeltaSeconds :type "Float (single-precision)"))
  (if (`self.isOverlapping`)
    (bind _ascaramuru (cast `/Game/Resources/Blueprints/Character/Caramuru` (`GameplayStatics.GetPlayerPawn` 0)))
    (if (`/Game/Resources/Blueprints/Character/Caramuru.ispress` _ascaramuru)
      (bind _key (`/Game/Resources/Blueprints/Character/Caramuru.key` _ascaramuru))
      (if (> _key 0)
        (set `/Game/Resources/Blueprints/Character/Caramuru.key` (- _key 1) _ascaramuru)
        (`self.K2_DestroyActor`)
        (`GameplayStatics.PlaySoundAtLocation` "/Game/Sounds/CUE_DoorUnlock.CUE_DoorUnlock")
        (else
          (`KismetSystemLibrary.PrintString` "Voce não tem uma chave"))))))

(event `self.Overlap.OnComponentBeginOverlap`
  (params (OverlappedComponent :type "PrimitiveComponent Object Reference") (OtherActor :type "Actor Object Reference") (OtherComp :type "PrimitiveComponent Object Reference") (OtherBodyIndex :type Integer) (bFromSweep :type Boolean) (SweepResult :type "HitResult Structure (by ref)"))
  (set `self.isOverlapping` true))

(event `self.Overlap.OnComponentEndOverlap`
  (params (OverlappedComponent :type "PrimitiveComponent Object Reference") (OtherActor :type "Actor Object Reference") (OtherComp :type "PrimitiveComponent Object Reference") (OtherBodyIndex :type Integer))
  (set `self.isOverlapping` false))

(fn `UserConstructionScript`)