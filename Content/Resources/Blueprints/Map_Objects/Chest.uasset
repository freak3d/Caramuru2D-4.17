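; Chest is an interactable map object that gives the Caramuru player a key when opened.
; Box overlap events set a flag, and Tick polls it along with the player's Ispress state.
; On opening, it increments the player's Key count, plays a sound at world origin, prints a Silver Key message, spawns Chest_Open at its location and destroys itself.
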(event `self.ReceiveTick`
  (params (DeltaSeconds :type "Float (single-precision)"))
  (if (`self.isOverlapping`)
    (bind _ascaramuru (cast `/Game/Resources/Blueprints/Character/Caramuru` (`GameplayStatics.GetPlayerPawn` 0)))
    (if (`/Game/Resources/Blueprints/Character/Caramuru.ispress` _ascaramuru)
      (set `/Game/Resources/Blueprints/Character/Caramuru.key` (+ (`/Game/Resources/Blueprints/Character/Caramuru.key` _ascaramuru) 1) _ascaramuru)
      (`GameplayStatics.PlaySoundAtLocation` "/Game/Sounds/CUE_ChestOpening.CUE_ChestOpening")
      (`KismetSystemLibrary.PrintString` "You receive 1 Silver Key.")
      (`|SpawnActorFromClass` "/Game/Resources/Blueprints/Map_Objects/Chest_Open.Chest_Open_C" (`KismetMathLibrary.Conv_VectorToTransform` (`self.K2_GetActorLocation`)) "Undefined" "OverrideRootScale" null null)
      (`self.K2_DestroyActor`))))

(event `self.Box.OnComponentBeginOverlap`
  (params (OverlappedComponent :type "PrimitiveComponent Object Reference") (OtherActor :type "Actor Object Reference") (OtherComp :type "PrimitiveComponent Object Reference") (OtherBodyIndex :type Integer) (bFromSweep :type Boolean) (SweepResult :type "HitResult Structure (by ref)"))
  (set `self.isOverlapping` true))

(event `self.Box.OnComponentEndOverlap`
  (params (OverlappedComponent :type "PrimitiveComponent Object Reference") (OtherActor :type "Actor Object Reference") (OtherComp :type "PrimitiveComponent Object Reference") (OtherBodyIndex :type Integer))
  (set `self.isOverlapping` false))

(fn `UserConstructionScript`)