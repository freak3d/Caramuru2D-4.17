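; Caramuru is the 2D Paper2D player character: it runs, jumps, climbs ladders, shoots, takes knockback hits and respawns.
; Each Tick, a CaramuruStates enum selects the sprite flipbook and checks for death and falling.
; Weapons cycle through a data table, tinting spawned BP_Shoot projectiles with the current color.
; Hits disable input and flag a dynamic sprite material until landing; death reloads the saved checkpoint position and restores life.
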(event `WeaponInit`
  (bind (_name _color _velocityx _velocityz _velocityzrange _scale _flipbook) (break `/Game/WeaponStructure` (`self.CurrentWeapon`)))
  ;[1 1 1] Weapon System
  (bind _outrownames (`DataTableFunctionLibrary.GetDataTableRowNames` "/Game/WeaponData.WeaponData"))
  (set `self.WeaponArray` _outrownames)
  (set `self.NumWeapons` (`KismetArrayLibrary.Array_LastIndex` _outrownames))
  (bind _output_get (set `self.WeaponIndex` (`KismetMathLibrary.Clamp` (+ (`self.WeaponIndex`) 1) 0 (`self.NumWeapons`)) :!label _label))
  (bind _returnvalue (`|GetDataTableRow` "/Game/WeaponData.WeaponData" (`|GetArrayItem` (`self.WeaponArray`) _output_get))
    (:`then`
      (set `self.CurrentWeapon` _returnvalue)
      (set `self.WeaponName` _name :!label _label_2)
      (set `self.WeaponColor` _color)
      (set `self.WeaponVelocityX` _velocityx)
      (set `self.WeaponVelocityZ` _velocityz)
      (set `self.WeaponVelocityZRange` _velocityzrange)
      (set `self.WeaponScale` _scale)
      (set `self.WeaponFlipbook` _flipbook)
      (`KismetSystemLibrary.PrintString` (`self.WeaponName`)))))

(event `InputAction|CicleWeaponUp`
  (params (Key :type "Key Structure"))
  ;[1 1 1] Weapon System
  (:`Pressed`
    (goto _label)))

(event `InputAction|Shoot`
  (params (Key :type "Key Structure"))
  ;[1 1 1] Shot
  (:`Pressed`
    (if (`self.isShoot`)
      (`GameplayStatics.PlaySoundAtLocation` "/Game/Sounds/CUE_ShootingSound.CUE_ShootingSound")
      (set `self.canMove` false)
      (set `self.CaramuruStates` "NewEnumerator7")
      (bind _returnvalue (`|SpawnActorFromClass` "/Game/Resources/Blueprints/Powers/BP_Shoot.BP_Shoot_C" (`SceneComponent.K2_GetComponentToWorld` (`self.Arrow1`)) "Undefined" "OverrideRootScale" null null))
      (`MaterialInstanceDynamic.SetVectorParameterValue` (`/Game/Resources/Blueprints/Powers/BP_Shoot.shootInstanceMaterial` _returnvalue) "Color" (`self.WeaponColor`))))
  (:`Released`
    (`KismetSystemLibrary.RetriggerableDelay` 0.3)
    (set `self.CaramuruStates` "NewEnumerator0")
    (set `self.canMove` true)))

(event `GroundEvent`
  ;[1 1 1] Shot
  (set `self.isGround` true)
  (set `self.canJump_0` true)
  (`CharacterMovementComponent.SetMovementMode` (`self.CharacterMovement`) "MOVE_Walking" 0))

(event `InputAction|CicleWeaponDown`
  (params (Key :type "Key Structure"))
  ;[1 1 1] Weapon System
  (:`Pressed`
    (bind _output_get (set `self.WeaponIndex` (`KismetMathLibrary.Clamp` (- (`self.WeaponIndex`) 1) 0 (`self.NumWeapons`))))
    (bind _returnvalue (`|GetDataTableRow` "/Game/WeaponData.WeaponData" (`|GetArrayItem` (`self.WeaponArray`) _output_get))
      (:`then`
        (set `self.CurrentWeapon` _returnvalue)
        (goto _label_2)))))

(event `Key|K`
  (params (Key :type "Key Structure"))
  ;[1 1 1] Shot
  (:`Pressed`
    (set `self.ispress` true)
    (`KismetSystemLibrary.Delay` 1e-06)
    (set `self.ispress` false :!label _label_3))
  (:`Released`
    (goto _label_3)))

(event `InputAxis|MoveUp`
  (params (AxisValue :type "Float (single-precision)"))
  ;[1 1 1] Climb
  ;;[0.222 0.1644 0.08874] Ladder Enter
  (if (`self.canClimb`)
    (if (not (`KismetMathLibrary.InRange_FloatFloat` AxisValue -0.001 0.001))
      (`CharacterMovementComponent.SetMovementMode` (`self.CharacterMovement`) "MOVE_Flying" 0)
      (`self.AddMovementInput` (`KismetMathLibrary.MakeVector` 0.0 0.0 (`self.climbSpeed`)) AxisValue)
      (set `self.isClimb` true)
      (set `self.isShoot` false)
      (set `self.canJump_0` false)
      (set `self.canMove` false))))

(event `self.ReceiveBeginPlay`
  ;[0.6459 0.4006 0.7396] Begin Play
  (`|ExecutionSequence`
    (:`then_0`
      (bind _returnvalue (`|CreateWidget` "/Game/Resources/hud.hud_C"))
      (`UserWidget.AddToViewport` _returnvalue 0)
      (`ActorComponent.SetIsReplicated` (`self.Sprite`) true))
    (:`then_1`
      (`self.WeaponInit`)
      (set `self.isShoot` true))))

(event `InputAction|Jump`
  (params (Key :type "Key Structure"))
  ;[1 0.206 0] Handle Jump
  (:`Pressed`
    (if (`self.isGround`)
      (if (`self.canJump_0`)
        (set `self.isGround` false)
        (set `self.isClimb` false)
        (`self.Jump`)
        (set `self.CaramuruStates` "NewEnumerator2")
        (set `self.isjumping` true))))
  (:`Released`
    (`self.StopJumping`)))

(event `self.ReceiveTick`
  (params (DeltaSeconds :type "Float (single-precision)"))
  ;[0 0 1] Tick - Updates animation
  (`self.UpdateAnimation`)
  (`self.Dead`)
  (`self.Falling`))

(event `ClimbEnd`
  ;[1 1 1] Climb
  ;;[0.09084 0.06663 0.0356] Ladder Exit
  (`CharacterMovementComponent.SetMovementMode` (`self.CharacterMovement`) "MOVE_Walking" 0)
  (set `self.isClimb` false))

(event `Direction`
  ;[1 1 0] Movement
  ;;[1 1 1] Direction
  (`SceneComponent.K2_SetRelativeRotation` (`self.Sprite`) (`KismetMathLibrary.MakeRotator` 0.0 0.0 (`KismetMathLibrary.SelectFloat` 0.0 180.0 (`self.bisMovingRight`))) false false))

(event `UpdateAnimation`
  (bind _returnvalue_x (`KismetMathLibrary.BreakVector` (`self.GetVelocity`)))
  (bind _sprite (`self.Sprite`))
  ;[0 1 1] Update Animation
  (switch `/Game/Caramuru-States` (`self.CaramuruStates`)
    (:`NewEnumerator0`
      (`PaperFlipbookComponent.SetFlipbook` _sprite (select `bool` (== (`KismetMathLibrary.VSize` (`KismetMathLibrary.MakeVector` _returnvalue_x)) 0.0) :`false` "/Game/Resources/2dtiledmap/CaramuruCharacter/CaramuruFlipBook/Walking/WALKING_Caramuru.WALKING_Caramuru" :`true` "/Game/Resources/2dtiledmap/CaramuruCharacter/IDLE_Caramuru.IDLE_Caramuru" :!type "PaperFlipbook Object Reference")))
    (:`NewEnumerator1`
      (`PaperFlipbookComponent.SetFlipbook` _sprite "/Game/Resources/2dtiledmap/CaramuruCharacter/CaramuruFlipBook/Walking/WALKING_Caramuru.WALKING_Caramuru"))
    (:`NewEnumerator2`
      (`PaperFlipbookComponent.SetFlipbook` _sprite "/Game/Resources/2dtiledmap/CaramuruCharacter/CaramuruFlipBook/Jumping/JUMPING_Caramuru.JUMPING_Caramuru"))
    (:`NewEnumerator3`
      (`PaperFlipbookComponent.SetFlipbook` _sprite "/Game/Char_Sprite/goku-dead.goku-dead"))
    (:`NewEnumerator5`
      (`PaperFlipbookComponent.SetFlipbook` _sprite "/Game/Char_Sprite/goku-hit.goku-hit"))
    (:`NewEnumerator6`
      (`PaperFlipbookComponent.SetFlipbook` _sprite "/Game/Char_Sprite/Goku_Sitting.Goku_Sitting"))
    (:`NewEnumerator7`
      (`PaperFlipbookComponent.SetFlipbook` _sprite "/Game/Resources/2dtiledmap/CaramuruCharacter/CaramuruFlipBook/Attacking/ATTACK_Caramuru.ATTACK_Caramuru"))
    (:`NewEnumerator8`
      (`PaperFlipbookComponent.SetFlipbook` _sprite "/Game/Resources/2dtiledmap/CaramuruCharacter/CaramuruFlipBook/Jumping/Caramuru_Falling.Caramuru_Falling"))))

(event `Hit`
  (params (NewParam :type "Float (double-precision)"))
  ;[1 0.07245 0.9595] Battle System
  ;;[0.51 0 0.00255] Hit
  (set `self.Life` NewParam)
  (set `self.isHit` true)
  (`GameplayStatics.PlaySoundAtLocation` "/Game/Sounds/CUE_Hit.CUE_Hit")
  (`self.DisableInput` (`GameplayStatics.GetPlayerController` 0))
  (set `self.CaramuruStates` "NewEnumerator5")
  (`CharacterMovementComponent.AddForce` (`self.CharacterMovement`) (`KismetMathLibrary.MakeVector` (* (`self.facing`) (`self.knockBack`)) 0.0 2500000.0))
  (`PrimitiveComponent.SetCollisionResponseToChannel` (`self.CapsuleComponent`) "ECC_GameTraceChannel1" "ECR_Ignore")
  (`MaterialInstanceDynamic.SetScalarParameterValue` (`self.spriteInstanceMaterial`) "isHit" 1.0))

(event `InputAxis|MoveRight`
  (params (AxisValue :type "Float (single-precision)"))
  ;[1 1 0] Movement
  ;;[1 1 1] Handle movement
  (if (`self.isClimb`)
    (if (`self.isGround`)
      (if (`self.canMove`) :!label _label_4
        (`self.Movement Right` AxisValue)
        (`self.Direction`)))
    (else
      (goto _label_4))))

(event `Dead`
  ;[1 0.07245 0.9595] Battle System
  ;;[0 0 0] Dead
  (if (<= (`self.Life`) 0.0)
    (set `self.isDead` true)
    (set `self.CaramuruStates` "NewEnumerator3")
    (`GameplayStatics.PlaySoundAtLocation` "/Game/Sounds/CUE_DIE.CUE_DIE")
    (`self.DisableInput` null)
    (`PrimitiveComponent.SetCollisionResponseToChannel` (`self.CapsuleComponent`) "ECC_GameTraceChannel1" "ECR_Ignore")
    (if (`self.isDead`)
      (bind _returnvalue (`GameplayStatics.LoadGameFromSlot` "Loc"))
      (bind _assave_info (cast `/Game/Resources/2dtiledmap/CheckPoint/Save_Info` _returnvalue))
      (`self.K2_SetActorRelativeLocation` (`/Game/Resources/2dtiledmap/CheckPoint/Save_Info.CheckLocation` _assave_info))
      (`CapsuleComponent.SetCapsuleHalfHeight` (`self.CapsuleComponent`) 18.0 true)
      (set `self.Life` 100.0)
      (`self.EnableInput` null)
      (set `self.CaramuruStates` "NewEnumerator0")
      (`PaperFlipbookComponent.Play` (`self.Sprite`))
      (set `self.isDead` false)
      (set `self.isHit` false)
      (`MaterialInstanceDynamic.SetScalarParameterValue` (`self.spriteInstanceMaterial`) "isHit" 0.0)
      (`PrimitiveComponent.SetCollisionResponseToChannel` (`self.CapsuleComponent`) "ECC_GameTraceChannel1" "ECR_Block"))))

(event `Movement Right`
  (params (MoveValue :type "Float (double-precision)"))
  ;[1 1 0] Movement
  ;;[1 1 1] isMovement
  (if (> MoveValue 0.0)
    (set `self.bisMovingRight` true)
    (set `self.facing` 1)
    (elif (< MoveValue 0.0)
      (set `self.bisMovingRight` false)
      (set `self.facing` -1)))
  (`self.AddMovementInput` (1.0 0.0 0.0) MoveValue))

(event `self.OnLanded`
  (params (Hit :type "HitResult Structure (by ref)"))
  ;[0.32 0.038 0] Ground Event
  (`self.GroundEvent`)
  (if (`self.isHit`)
    (if (`self.isDead`)
      (set `self.CaramuruStates` "NewEnumerator3")
      (else
        (set `self.CaramuruStates` "NewEnumerator6")
        (`KismetSystemLibrary.Delay` 0.7)
        (set `self.isHit` false)
        (set `self.CaramuruStates` "NewEnumerator0")
        (`self.EnableInput` (`GameplayStatics.GetPlayerController` 0))
        (`PrimitiveComponent.SetCollisionResponseToChannel` (`self.CapsuleComponent`) "ECC_GameTraceChannel1" "ECR_Block")
        (`MaterialInstanceDynamic.SetScalarParameterValue` (`self.spriteInstanceMaterial`) "isHit" 0.0)))
    (else
      (set `self.CaramuruStates` "NewEnumerator0")
      (set `self.isjumping` false)
      (`self.GroundEvent`))))

(event `Falling`
  ;[1 1 1] Fall
  (if (`NavMovementComponent.IsFalling` (`self.CharacterMovement`))
    (set `self.isFalling` true)
    (set `self.CaramuruStates` "NewEnumerator8")))

(fn `UserConstructionScript`
  (bind _returnvalue (`PrimitiveComponent.CreateDynamicMaterialInstance` (`self.Sprite`) 0 "/Game/Sprite_material.Sprite_Material"))
  (set `self.spriteInstanceMaterial` _returnvalue))